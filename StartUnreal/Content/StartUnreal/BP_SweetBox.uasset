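; BP_SweetBox is a trigger box that starts and stops event behavior on actors throughout the level when anything overlaps its Cube.
; Begin and end overlap each print debug names, both labeled "Begin Overlap", then scan every Actor for an EventComponent.
; Each component found receives DoPlay on begin and DoStop on end.
; An alternative broadcast through the BPI_Event interface is present but never runs.
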(event OnComponentBeginOverlap(Cube)
  (params (OverlappedComponent :type Primitive%20Component%20Object%20Reference) (OtherActor :type Actor%20Object%20Reference) (OtherComp :type Primitive%20Component%20Object%20Reference) (OtherBodyIndex :type Integer) (bFromSweep :type Boolean) (SweepResult :type Hit%20Result%20Structure%20%28by%20ref%29))
  (Development|PrintString (Utilities|String|Append "Begin Overlap " (Utilities|GetDisplayName OverlappedComponent) "Other Actor" (Utilities|GetDisplayName OtherActor) "Other Component" (Utilities|GetDisplayName OtherComp)))
  (bind _outactors (Actor|GetAllActorsOfClass "/Script/Engine.Actor"))
  (for _array_element _outactors
    (Utilities|IsValid (Actor|GetComponentbyClass _array_element "/Game/StartUnreal/EventComponent.EventComponent_C")
      (:Is%20Valid
        (Default|DoPlay (Actor|GetComponentbyClass _array_element "/Game/StartUnreal/EventComponent.EventComponent_C"))))))

(event OnComponentEndOverlap(Cube)
  (params (OverlappedComponent :type Primitive%20Component%20Object%20Reference) (OtherActor :type Actor%20Object%20Reference) (OtherComp :type Primitive%20Component%20Object%20Reference) (OtherBodyIndex :type Integer))
  (Development|PrintString (Utilities|String|Append "Begin Overlap " (Utilities|GetDisplayName OverlappedComponent) "Other Actor" (Utilities|GetDisplayName OtherActor) "Other Component" (Utilities|GetDisplayName OtherComp)))
  (bind _outactors (Actor|GetAllActorsOfClass "/Script/Engine.Actor"))
  (for _array_element _outactors
    (Utilities|IsValid (Actor|GetComponentbyClass _array_element "/Game/StartUnreal/EventComponent.EventComponent_C")
      (:Is%20Valid
        (Default|DoStop (Actor|GetComponentbyClass _array_element "/Game/StartUnreal/EventComponent.EventComponent_C"))))))

(fn ConstructionScript)