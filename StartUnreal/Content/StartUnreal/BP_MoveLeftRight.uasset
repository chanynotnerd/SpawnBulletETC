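; BP_MoveLeftRight is an actor that slides its Sphere component back and forth along its relative X axis.
; While IsPlay is true, Tick steps the offset by a fixed amount per frame without delta time, so speed depends on frame rate.
; IsMoveRight flips whenever the offset passes either end of a short fixed range.
; EventComponent's DoPlay and DoStop dispatchers start and pause the motion by setting IsPlay.
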(event EventDispatcherDoPlay(EventComponent)
  (Variables|Default|SetIsPlay true))

(event EventDispatcherDoStop(EventComponent)
  (Variables|Default|SetIsPlay false))

(event EventTick
  (params (DeltaSeconds :type Float%20%28single-precision%29))
  (if (Variables|Default|GetIsPlay)
    ;[1 1 1] If문을 통해 방향 지정
    (if (Variables|Default|GetIsMoveRight)
      ;[1 1 1] 오른쪽 이동
      (Variables|Default|SetSomething (+ 1.0 (Variables|Default|GetSomething)))
      (Transformation|SetRelativeLocation (Variables|Default|GetSphere) (Math|Vector|MakeVector (Variables|Default|GetSomething) 0.0 0.0) false false)
      ;[1 1 1] 방향을 바꿔주기 위함
      (if (> (Variables|Default|GetSomething) 1e+02)
        (Variables|Default|SetIsMoveRight false))
      (else
        ;[1 1 1] 뒤로 이동
        (Variables|Default|SetSomething (- (Variables|Default|GetSomething) 1.0))
        (Transformation|SetRelativeLocation (Variables|Default|GetSphere) (Math|Vector|MakeVector (Variables|Default|GetSomething) 0.0 0.0) false false)
        ;[1 1 1] 방향을 바꿔주기 위함
        (if (< (Variables|Default|GetSomething) 0.0)
          (Variables|Default|SetIsMoveRight true))))))

(fn ConstructionScript)